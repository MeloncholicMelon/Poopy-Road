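; BP_TileRow is an actor that builds a row of tiles centred on its origin along local X.
; The construction script destroys the root's child components, then adds NumberOfTiles child actor components of class Tile.
; Alternating sign and a rounded-up half index place tiles outward on both sides at fixed spacing.
; The event graph holds only disabled events and an unconnected player-position check that would print a win message.
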(event Collision|EventActorBeginOverlap
  (params (OtherActor :type Actor%20Object%20Reference)))

(event EventTick
  (params (DeltaSeconds :type Float%20%28single-precision%29)))

(fn ConstructionScript
  ;[1 1 1] Destroy the present components
  (for _array_element (Components|GetChildrenComponents (Variables|Default|GetDefaultSceneRoot) false)
    (Components|DestroyComponent _array_element))
  ;[1 1 1] Create a row of tiles
  (for _index (range 0 (- (Variables|Default|GetNumberOfTiles) 1))
    (bind _returnvalue (AddComponent|AddChildActorComponent false (Math|Transform|MakeTransform (Math|Vector|MakeVector (* (Math|Float|Power -1.0 (Math|Conversions|ToFloat(Integer) _index)) 1e+02 (Math|Conversions|ToFloat(Integer) (Math|Float|Ceil (/ (Math|Conversions|ToFloat(Integer) _index) 2.0)))) 0.0 0.0))))
    (ChildActorComponent|SetChildActorClass _returnvalue (Variables|Default|GetTile))))