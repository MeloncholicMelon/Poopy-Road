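; Player actor for a hop-to-the-goal game, moving in fixed steps along X and Y with WASD.
; Each key sets a target that a shared timeline reaches by swept lerp from the current location.
; Tick scores each new furthest target Y and prints a win past a distance threshold, while any overlap destroys the player and prints game over.
; The construction script applies configurable body and head meshes.
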(event EventBeginPlay
  (bind _returnvalue (Transformation|GetActorLocation))
  (Variables|Default|Settarget%20location _returnvalue)
  (Variables|Default|SetmaxY _returnvalue))

(event Collision|EventActorBeginOverlap
  (params (OtherActor :type Actor%20Object%20Reference))
  (Actor|DestroyActor)
  (Development|PrintString "Game Over!")
  (Development|PrintString (Utilities|String|ToString(Integer) (Variables|Default|Getscore))))

(event EventTick
  (params (DeltaSeconds :type Float%20%28single-precision%29))
  (if (> (.Y (Math|Vector|BreakVector (Variables|Default|Gettarget%20location))) (.Y (Math|Vector|BreakVector (Variables|Default|GetmaxY))))
    (Variables|Default|Setscore (+ (Variables|Default|Getscore) 1))
    (Variables|Default|SetmaxY (Variables|Default|Gettarget%20location))
    (if (>= (.Y (Math|Vector|BreakVector (Variables|Default|Gettarget%20location))) 6e+03)
      (Development|PrintString "You Won! Score:")
      (Development|PrintString (Utilities|String|ToString(Integer) (Variables|Default|Getscore))))))

(event Input|KeyboardEvents|W
  (params (Key :type Key%20Structure :default "None"))
  (bind _returnvalue (Transformation|GetActorLocation))
  (:Pressed
    (Variables|Default|Settarget%20location (+ "0,100.000000,0.000000" _returnvalue))
    (bind _newtrack_0 (Timeline|Timeline_0 PlayFromStart)
      (:Update
        (Transformation|SetActorLocation (Math|Vector|Lerp(Vector) _returnvalue (Variables|Default|Gettarget%20location) _newtrack_0) true false)))))

(event Input|KeyboardEvents|S
  (params (Key :type Key%20Structure :default "None"))
  (bind _returnvalue (Transformation|GetActorLocation))
  (:Pressed
    (Variables|Default|Settarget%20location (+ "0,-100.000000, 0" _returnvalue))
    (bind _newtrack_0 (Timeline|Timeline_0 PlayFromStart)
      (:Update
        (Transformation|SetActorLocation (Math|Vector|Lerp(Vector) _returnvalue (Variables|Default|Gettarget%20location) _newtrack_0) true false)))))

(event Input|KeyboardEvents|A
  (params (Key :type Key%20Structure :default "None"))
  (bind _returnvalue (Transformation|GetActorLocation))
  (:Pressed
    (Variables|Default|Settarget%20location (+ "100.000000,0.000000, 0" _returnvalue))
    (bind _newtrack_0 (Timeline|Timeline_0 PlayFromStart)
      (:Update
        (Transformation|SetActorLocation (Math|Vector|Lerp(Vector) _returnvalue (Variables|Default|Gettarget%20location) _newtrack_0) true false)))))

(event Input|KeyboardEvents|D
  (params (Key :type Key%20Structure :default "None"))
  (bind _returnvalue (Transformation|GetActorLocation))
  (:Pressed
    (Variables|Default|Settarget%20location (+ "-100.000000,0.000000, 0" _returnvalue))
    (bind _newtrack_0 (Timeline|Timeline_0 PlayFromStart)
      (:Update
        (Transformation|SetActorLocation (Math|Vector|Lerp(Vector) _returnvalue (Variables|Default|Gettarget%20location) _newtrack_0) true false)))))

(fn ConstructionScript
  (Components|StaticMesh|SetStaticMesh (Variables|Default|GetBody) (Variables|Default|GetBodyModel))
  (Components|StaticMesh|SetStaticMesh (Variables|Default|GetHead) (Variables|Default|GetHeadModel)))